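; BP_ScoresList is a level scoreboard that records the player's goals and prints all scores on screen at BeginPlay.
; SaveCurrentScore adds the third-person character's name and goals to a name-keyed map; after ten names, it removes lower-scoring entries before adding.
; GetScoresList formats the map as "name-score" strings for long-duration text printing.
; Scores live only in Blueprint variables, without SaveGame, and OrderNames is an empty stub.
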(event EventBeginPlay
  (CallFunction|SaveCurrentScore)
  (bind _finallist (CallFunction|GetScoresList))
  (for _array_element _finallist
    (Development|PrintText (Utilities|Text|ToText(String) _array_element) true true "(R=0.000000,G=0.660000,B=1.000000,A=1.000000)" 1.8e+05)))

(fn ConstructionScript)

(fn GetScoresList
  (bind _scores (Variables|Default|GetScores))
  (bind _finallist (Variables|Default|GetFinalList))
  (bind _keys (Utilities|Map|Keys _scores))
  (for _array_element _keys
    (Utilities|Array|Add _finallist (Utilities|String|Append (Utilities|String|Append _array_element " - ") (Utilities|String|ToString(Integer) (.Value (Utilities|Map|Find _scores _array_element))))))
  (return _finallist))

(fn SaveCurrentScore
  (bind _scores (Variables|Default|GetScores))
  (bind _asbp_third_person_character (Utilities|Casting|CastToBP_ThirdPersonCharacter (Game|GetPlayerCharacter 0)))
  (if (< (Utilities|Array|Length (Variables|Default|GetNames)) 10)
    (Utilities|Array|Add (Variables|Default|GetNames) (Variables|/Game/ThirdPerson/Blueprints/BP_ThirdPersonCharacter.BP_ThirdPersonCharacter_C|GetName _asbp_third_person_character) :!label _label)
    (Utilities|Map|Add (Variables|Default|GetScores) (Variables|/Game/ThirdPerson/Blueprints/BP_ThirdPersonCharacter.BP_ThirdPersonCharacter_C|GetName _asbp_third_person_character) (Variables|/Game/ThirdPerson/Blueprints/BP_ThirdPersonCharacter.BP_ThirdPersonCharacter_C|GetGoals _asbp_third_person_character))
    (else
      (bind _keys (Utilities|Map|Keys _scores))
      (for _array_element _keys
        (if (< (.Value (Utilities|Map|Find _scores _array_element)) (Variables|/Game/ThirdPerson/Blueprints/BP_ThirdPersonCharacter.BP_ThirdPersonCharacter_C|GetGoals _asbp_third_person_character))
          (Utilities|Map|Remove (Variables|Default|GetScores) _array_element)
          (goto _label))))))

(fn OrderNames
  (params (Input :type Array%20of%20Strings)))