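; Player actor for the start-screen menu that swings its CineCamera between two yaw angles and hides the mouse cursor on BeginPlay.
; Tick checks the Controles flag, which is not set in this graph, and plays one of two timelines that lerp the camera's relative yaw in opposite directions across a quarter turn.
; Both timelines use Play rather than PlayFromStart, and neither is reset here.
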(event EventBeginPlay
  (Variables|/Script/Engine.PlayerController|SetbShowMouseCursor (Game|GetPlayerController 0) false))

(event Collision|EventActorBeginOverlap
  (params (OtherActor :type Actor%20Object%20Reference)))

(event EventTick
  (params (DeltaSeconds :type Float%20%28single-precision%29))
  (if (Variables|Default|Getcontroles)
    (bind _rotar (Timeline|Rota Play)
      (:Update
        (Transformation|SetRelativeRotation (Variables|Default|GetCineCamera) (Math|Rotator|MakeRotator 0.0 0.0 (Math|Float|Lerp 9e+01 0.0 (.z _rotar))) false false)))
    (else
      (bind _rotar_2 (Timeline|Línea%20de%20tiempo Play)
        (:Update
          (Transformation|SetRelativeRotation (Variables|Default|GetCineCamera) (Math|Rotator|MakeRotator 0.0 0.0 (Math|Float|Lerp 0.0 9e+01 (.z _rotar_2))) false false))))))

(fn ConstructionScript)