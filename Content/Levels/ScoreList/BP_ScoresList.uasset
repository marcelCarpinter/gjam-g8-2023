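; BP_ScoresList keeps a score table of player names and goal counts for a leaderboard-style list.
; SaveCurrentScore records the third-person character's Name and Goals in a map when Goals exceeds a fixed threshold.
; GetScoresList appends each entry to FinalList as a "score-name" string and returns it.
; SortArray is a separate swap-based string sort comparing character codes, so numbers order as text; nothing here calls it.
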(fn ConstructionScript)

(fn GetScoresList
  (bind _scores (Variables|Default|GetScores))
  (bind _finallist (Variables|Default|GetFinalList))
  (bind _keys (Utilities|Map|Keys _scores))
  (for _array_element _keys
    (Utilities|Array|Add _finallist (Utilities|String|Append (Utilities|String|Append (Utilities|String|ToString(Integer) (.Value (Utilities|Map|Find _scores _array_element))) " - ") _array_element)))
  (return _finallist))

(fn SaveCurrentScore
  (bind _asbp_third_person_character (Utilities|Casting|CastToBP_ThirdPersonCharacter (Game|GetPlayerCharacter 0)))
  (if (> (Variables|/Game/ThirdPerson/Blueprints/BP_ThirdPersonCharacter.BP_ThirdPersonCharacter_C|GetGoals _asbp_third_person_character) 12)
    (Utilities|Array|Add (Variables|Default|GetNames) (Variables|/Game/ThirdPerson/Blueprints/BP_ThirdPersonCharacter.BP_ThirdPersonCharacter_C|GetName _asbp_third_person_character))
    (Utilities|Map|Add (Variables|Default|GetScores) (Variables|/Game/ThirdPerson/Blueprints/BP_ThirdPersonCharacter.BP_ThirdPersonCharacter_C|GetName _asbp_third_person_character) (Variables|/Game/ThirdPerson/Blueprints/BP_ThirdPersonCharacter.BP_ThirdPersonCharacter_C|GetGoals _asbp_third_person_character))))

(fn SortArray
  (params (ArrayToSort :type Array%20of%20Strings))
  (Variables|Default|SetArraytoSort ArrayToSort)
  (Variables|Default|SetAscending true)
  (for (_array_element _array_index) (Variables|Default|GetArraytoSort)
    (for _index (range _array_index (Utilities|Array|LastIndex (Variables|Default|GetArraytoSort)))
      (bind _index_2 (Utilities|FlowControl|ForLoopwithBreak 0 (- (select (> (Utilities|String|Len (Utilities|Array|Get(acopy) (Variables|Default|GetArraytoSort) _index)) (Utilities|String|Len _array_element)) (Utilities|String|Len _array_element) (Utilities|String|Len (Utilities|Array|Get(acopy) (Variables|Default|GetArraytoSort) _index))) 1) :!label _label)
        (:LoopBody
          (if (!= (Utilities|String|GetCharacterasNumber (Utilities|Array|Get(acopy) (Variables|Default|GetArraytoSort) _index) _index_2) (Utilities|String|GetCharacterasNumber _array_element _index_2))
            (goto _label Break)))
        (:Completed
          (if (Variables|Default|GetAscending)
            (if (> (Utilities|String|GetCharacterasNumber (Utilities|Array|Get(acopy) (Variables|Default|GetArraytoSort) _index) _index_2) (Utilities|String|GetCharacterasNumber _array_element _index_2))
              (Utilities|Array|Swap ArrayToSort _index _array_index :!label _label_2))
            (elif (< (Utilities|String|GetCharacterasNumber (Utilities|Array|Get(acopy) (Variables|Default|GetArraytoSort) _index) _index_2) (Utilities|String|GetCharacterasNumber _array_element _index_2))
              (goto _label_2)))))))
  (return ArrayToSort))