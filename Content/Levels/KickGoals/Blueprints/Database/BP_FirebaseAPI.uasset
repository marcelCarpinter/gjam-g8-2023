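; Firebase API blueprint for the KickGoals level that fetches stored scores over REST.
; GetScores sends a JSON GET request to the URL variable through the VaRest subsystem.
; The Response callback walks the nested typed-field JSON (list, arrayValue, mapValue) and prints the score and name of the first entry only as on-screen debug text.
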(event Custom|Response
  (params (Request :type Va%20Rest%20Request%20JSON%20Object%20Reference))
  (bind _returnvalue (Class|VaRestJsonValue|AsObject (Utilities|Array|Get(acopy) (Class|VaRestJsonObject|GetArrayField (Class|VaRestJsonObject|GetObjectField (Class|VaRestJsonObject|GetObjectField (Class|VaRestJsonObject|GetObjectField (Class|VaRestRequestJSON|GetResponseObject Request) "fields") "list") "arrayValue") "values"))))
  (Development|PrintString (Class|VaRestJsonObject|GetStringField (Class|VaRestJsonObject|GetObjectField (Class|VaRestJsonObject|GetObjectField (Class|VaRestJsonObject|GetObjectField _returnvalue "mapValue") "fields") "score") "integerValue") true true "(R=1.000000,G=0.000000,B=0.214379,A=1.000000)" 1.8e+03)
  (Development|PrintString (Class|VaRestJsonObject|GetStringField (Class|VaRestJsonObject|GetObjectField (Class|VaRestJsonObject|GetObjectField (Class|VaRestJsonObject|GetObjectField _returnvalue "mapValue") "fields") "name") "stringValue") true true "(R=0.000000,G=0.390625,B=0.030963,A=1.000000)" 1.8e+03))

(event Custom|GetScores
  (Class|VaRestSubsystem|CallURL (|VaRestSubsystem) (Variables|Default|GetURL) "GET" "json" 0 (delegate Custom|Response)))

(fn ConstructionScript)