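; SoccerBallCollision is an out-of-bounds barrier for the KickGoals level that penalizes the player when a soccer ball enters it.
; It caches the third-person character on BeginPlay, then decrements that character's Hearts whenever a SoccerBall overlaps the collision component.
; With hearts left, it plays an error sound, destroys the ball and has BP_BallSpawner spawn a replacement.
; At zero, it pauses the game and shows the game-over widget with the mouse cursor.
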(event OnComponentBeginOverlap(OutOfBoundsCollision)
  (params (OverlappedComponent :type Primitive%20Component%20Object%20Reference) (OtherActor :type Actor%20Object%20Reference) (OtherComp :type Primitive%20Component%20Object%20Reference) (OtherBodyIndex :type Integer) (bFromSweep :type Boolean) (SweepResult :type Hit%20Result%20Structure%20%28by%20ref%29))
  (bind _assoccer_ball (Utilities|Casting|CastToSoccerBall OtherActor))
  (bind _result (Math|Integer|DecrementInt (Variables|/Game/ThirdPerson/Blueprints/BP_ThirdPersonCharacter.BP_ThirdPersonCharacter_C|GetHearts (Variables|Default|GetPlayer)))
    (:%20%20
      (if (<= _result 0)
        (Game|SetGamePaused true)
        (Variables|/Script/Engine.PlayerController|SetbShowMouseCursor (Game|GetPlayerController 0) true)
        (bind _returnvalue (UserInterface|CreateWidget "/Game/Levels/Dev_Level_Franco/Menu/BPW_GameOver_Screen.BPW_GameOver_Screen_C"))
        (UserInterface|Viewport|AddtoViewport _returnvalue 0)
        (else
          (Audio|Components|Audio|Play (Variables|Default|GetErrorSound) 0.0)
          (Actor|DestroyActor _assoccer_ball)
          (CallFunction|GetBalltoSpawn))))))

(event Custom|GetBallToSpawn
  (bind _returnvalue (Actor|GetActorOfClass "/Game/Levels/KickGoals/Blueprints/Spawner/BP_BallSpawner.BP_BallSpawner_C"))
  (Default|SpawnBasicBall _returnvalue))

(event EventBeginPlay
  (bind _asbp_third_person_character (Utilities|Casting|CastToBP_ThirdPersonCharacter (Game|GetPlayerCharacter 0)))
  (Variables|Default|SetPlayer _asbp_third_person_character))

(fn ConstructionScript)