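; Soccer goal target for the KickGoals level that translates along the world X axis on a timeline.
; AddSoccerGoal takes a distance, and GetMovingDistance turns any positive value into fixed endpoints either side of the actor's location.
; The distance also sets MovingRate, so larger values slow the timeline that lerps the actor between those endpoints.
; BeginPlay passes zero, which gives no offset.
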(event Custom|AddSoccerGoal
  (params (Distance :type Integer))
  (bind _moveinline (Variables|Default|GetMoveInLine))
  (bind _returnvalue (Components|Timeline|GetTimelineLength _moveinline))
  (bind (_start _end) (CallFunction|GetMovingDistance (Math|Conversions|ToFloat(Integer) Distance)))
  (Components|Timeline|SetPlayRate _moveinline (/ _returnvalue (* _returnvalue (Variables|Default|GetMovingRate))))
  (bind _float_track (Timeline|MoveInLine Play)
    (:Update
      (Transformation|SetActorLocation (Math|Vector|Lerp(Vector) _start _end _float_track) false false))))

(event EventBeginPlay
  (CallFunction|AddSoccerGoal))

(fn ConstructionScript
  (|CallParentFunction))

(fn GetMovingDistance
  (params (Distance :type Float%20%28double-precision%29))
  (bind _returnvalue (Transformation|GetActorLocation))
  (if (> Distance 0.0)
    (Variables|Default|SetAddedDistance "1000.000000,0.000000,0.000000")
    (else
      (Variables|Default|SetAddedDistance "0, 0, 0")))
  (Utilities|FlowControl|Sequence
    (:then_0
      (Variables|Default|SetMovingRate (/ Distance 2.0))
      (bind _output_get (Variables|Default|SetStartLocation (+ _returnvalue (* (Variables|Default|GetAddedDistance) -1))))
      (bind _output_get_2 (Variables|Default|SetEndLocation (+ _returnvalue (Variables|Default|GetAddedDistance))))
      (return _output_get _output_get_2))))