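; BP_TargetMovement is a target for the KickGoals level that moves along a straight line on the world X axis, centered on its placed position.
; On BeginPlay it stores endpoints either side of that position, and a timeline lerps the actor between them without sweeping.
; The timeline play rate is the inverse of MovingRate.
; A custom event reduces MovingRate and reapplies the rate, speeding up the target by ten percent per call.
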(event Custom|CustomEvent
  (bind _moveinline (Variables|Default|GetMoveInLine))
  (bind _returnvalue (Components|Timeline|GetTimelineLength _moveinline))
  (Variables|Default|SetMovingRate (/ (Variables|Default|GetMovingRate) 1.1))
  (Components|Timeline|SetPlayRate _moveinline (/ _returnvalue (* _returnvalue (Variables|Default|GetMovingRate))))
  (bind _float_track (Timeline|Timeline Play)
    (:Update
      (Transformation|SetActorLocation (Math|Vector|Lerp(Vector) (stale EventBeginPlay _output_get) (stale EventBeginPlay _output_get_2) _float_track) false false))))

(event EventBeginPlay
  (bind _returnvalue (Transformation|GetActorLocation))
  (bind _moveinline (Variables|Default|GetMoveInLine))
  (bind _returnvalue_2 (Components|Timeline|GetTimelineLength _moveinline))
  (bind _output_get (Variables|Default|SetStartLocation (+ _returnvalue "-2000.000000,0.000000,0.000000")))
  (bind _output_get_2 (Variables|Default|SetEndLocation (+ _returnvalue "2000.000000,0.000000,0.000000")))
  (Components|Timeline|SetPlayRate _moveinline (/ _returnvalue_2 (* _returnvalue_2 (Variables|Default|GetMovingRate))))
  (bind _float_track (Timeline|Timeline Play)
    (:Update
      (Transformation|SetActorLocation (Math|Vector|Lerp(Vector) _output_get _output_get_2 _float_track) false false))))

(fn ConstructionScript
  (|CallParentFunction))