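; BP_SoccerGoal is the soccer goal for the KickGoals level, scoring a point when a SoccerBall overlaps its collision.
; A score increments the player's goal count, plays sounds, and grants a heart every third goal while below the cap.
; It then destroys the ball, requests another from BP_BallSpawner, and updates itself by casting to its Translate or Rotate subclass to adjust movement.
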(event OnComponentBeginOverlap(GoalCollission)
  (params (OverlappedComponent :type Primitive%20Component%20Object%20Reference) (OtherActor :type Actor%20Object%20Reference) (OtherComp :type Primitive%20Component%20Object%20Reference) (OtherBodyIndex :type Integer) (bFromSweep :type Boolean) (SweepResult :type Hit%20Result%20Structure%20%28by%20ref%29))
  (bind _assoccer_ball (Utilities|Casting|CastToSoccerBall OtherActor))
  (Variables|Default|SetAs%20Soccer%20Ball _assoccer_ball)
  (bind _outactors (Actor|GetAllActorsOfClass "/Game/ThirdPerson/Blueprints/BP_ThirdPersonCharacter.BP_ThirdPersonCharacter_C"))
  (bind _output_get (Variables|Default|SetPlayer (Utilities|Array|Get(acopy) _outactors)))
  (bind _result (Math|Integer|IncrementInt (Variables|/Game/ThirdPerson/Blueprints/BP_ThirdPersonCharacter.BP_ThirdPersonCharacter_C|GetGoals _output_get))
    (:%20%20
      (Audio|Components|Audio|Play (Variables|Default|GetGoalSound) 0.0)
      (if (and (== (Math|Integer|%(Integer) _result 3) 0) (< (Variables|/Game/ThirdPerson/Blueprints/BP_ThirdPersonCharacter.BP_ThirdPersonCharacter_C|GetHearts _output_get) 5))
        (Math|Integer|IncrementInt (Variables|/Game/ThirdPerson/Blueprints/BP_ThirdPersonCharacter.BP_ThirdPersonCharacter_C|GetHearts _output_get)
          (:%20%20
            (Audio|Components|Audio|Play (Variables|Default|GetLifeUpSound) 0.0))))
      (Actor|DestroyActor (Variables|Default|GetAs%20Soccer%20Ball))
      (CallFunction|GetBalltoSpawn)
      (if (and (> _result 0) (== (Variables|Default|GetMovingRate) 0.0))
        (Variables|Default|SetMovingRate 2.0))
      (CallFunction|UpdateSoccerGoal))))

(event OnComponentEndOverlap(GoalCollission)
  (params (OverlappedComponent :type Primitive%20Component%20Object%20Reference) (OtherActor :type Actor%20Object%20Reference) (OtherComp :type Primitive%20Component%20Object%20Reference) (OtherBodyIndex :type Integer)))

(event Custom|GetBallToSpawn
  (if (> 5000000 (Variables|/Game/ThirdPerson/Blueprints/BP_ThirdPersonCharacter.BP_ThirdPersonCharacter_C|GetGoals (Variables|Default|GetPlayer)))
    (bind _returnvalue (Actor|GetActorOfClass "/Game/Levels/KickGoals/Blueprints/Spawner/BP_BallSpawner.BP_BallSpawner_C"))
    (Default|SpawnBasicBall _returnvalue)))

(event Custom|GetSoccerGoalToSpawn
  (bind _returnvalue (Actor|GetActorOfClass "/Game/Levels/KickGoals/Blueprints/Spawner/BP_TargetSpawner.BP_TargetSpawner_C"))
  (bind _soccergoal (Default|SpawnStaticTarget _returnvalue))
  (Default|AddSoccerGoal _soccergoal 0.0))

(event Custom|UpdateSoccerGoal
  (bind _self self)
  (bind _asbp_soccer_goal_translate (Utilities|Casting|CastToBP_SoccerGoal_Translate _self)
    (:then
      (Default|AddSoccerGoal _asbp_soccer_goal_translate (Variables|Default|GetMovingRate)))
    (:CastFailed
      (bind _asbp_soccer_goal_rotate (Utilities|Casting|CastToBP_SoccerGoal_Rotate _self))
      (Default|RotateGoal _asbp_soccer_goal_rotate (Variables|/Game/ThirdPerson/Blueprints/BP_ThirdPersonCharacter.BP_ThirdPersonCharacter_C|GetGoals (Variables|Default|GetPlayer))))))

(fn ConstructionScript)